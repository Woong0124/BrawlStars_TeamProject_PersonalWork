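; Player character Lou, with cursor-aimed Q, W and E skills.
; Q turns Lou toward the cursor and spawns two delayed successive shots from the arrow point.
; W launches an actor that Tick destroys near the saved cursor point, spawning blizzard Niagara effects and a collision actor there.
; E toggles movement off and its effect on, using gates to block Q and W meanwhile.
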(event `Key|Q`
  (params (Key :type "Key Structure"))
  ;[1 1 1] Q Skill
  (:`Pressed`
    (`self.E_SkillQ`)))

(event `E_SkillQ`
  (`/Engine/EditorBlueprintResources/StandardMacros.Gate` false :!label _label
    (:`Exit`
      (`self.AllSpawnSkill` (`self.C_RefSkillQ`) (`self.SkillArrowPoint`))
      (`KismetSystemLibrary.Delay` 0.2)
      (`self.TurnActor`)
      (`self.SpawnSkill_Target_ver` (`self.C_RefSkillQ`) (`self.SkillArrowPoint`)))))

(event `Key|E`
  (params (Key :type "Key Structure"))
  ;[1 1 1] E Skill
  (:`Pressed`
    (`self.E_SkillE`)))

(event `E_SkillE`
  (`NavMovementComponent.StopActiveMovement` (`self.CharacterMovement`))
  (if (`ActorComponent.IsActive` (`self.CharacterMovement`))
    (bind _output_get (set `self.bSkillE_Visibility` true))
    (`self.SkillVisibility` _output_get)
    (`|ExecutionSequence`
      (:`then_0`
        (goto _label :!via `Close`))
      (:`then_1`
        (goto _label_2 :!via `Close`)))
    (else
      (bind _output_get_2 (set `self.bSkillE_Visibility` false))
      (`self.SkillVisibility` _output_get_2)
      (`|ExecutionSequence`
        (:`then_0`
          (goto _label :!via `Open`))
        (:`then_1`
          (goto _label_2 :!via `Open`))))))

(event `Key|W`
  (params (Key :type "Key Structure"))
  ;[1 1 1] W Skill
  (:`Pressed`
    (`self.E_SkillW`)))

(event `E_SkillW`
  (`/Engine/EditorBlueprintResources/StandardMacros.Gate` false :!label _label_2
    (:`Exit`
      (bind _location (`self.SaveCursorToWorld`))
      (set `self.SaveParticleSpawnPoint` _location)
      (bind _spawnskillreturnvalue (`self.AllSpawnSkill` (`self.C_RefSkillW`) (`self.SkillArrowPoint`)))
      (set `self.SkillW` _spawnskillreturnvalue))))

(event `E_SkillW_Particle`
  (params (SpawnLocation :type "Vector Structure"))
  ;[1 1 1] Lou Skill W 나이아가라 파티클 생성
  (`self.SpawnSkillParticle` SpawnLocation "/Game/__OWNER/Woong/FX/NP_LouSkillW_Blizzard.NP_LouSkillW_Blizzard" "/Game/__OWNER/Woong/FX/NP_LouSkillW_Ground.NP_LouSkillW_Ground" "/Game/__OWNER/Woong/FX/NP_LouSkillW_Smoke.NP_LouSkillW_Smoke")
  (`self.E_SkillW_Collision` SpawnLocation))

(event `self.ReceiveTick`
  (params (DeltaSeconds :type "Float (single-precision)"))
  (bind _skillw (`self.SkillW`))
  (bind _returnvalue (`self.K2_GetActorLocation` _skillw))
  ;[1 1 1] Tick
  (`|ExecutionSequence`
    (:`then_0`
      ;[1 1 1] W 활성화 시, 실행
      (`/Engine/EditorBlueprintResources/StandardMacros.IsValid` _skillw
        (:`Is Valid`
          (if (== _returnvalue (`self.SaveParticleSpawnPoint`) :`ErrorTolerance` 80.0)
            (bind _output_get (set `self.SaveParticleSpawnPoint` _returnvalue))
            (`self.E_SkillW_Particle` _output_get)
            (`self.K2_DestroyActor` (`self.SkillW`))))))
    (:`then_1`
      ;[1 1 1] 커서의 위치를 저장
      (`self.SaveCursorToWorld`)
      (`SkinnedMeshComponent.HideBoneByName` (`self.Mesh`) "L_gunbone_01_s" "PBO_Term"))))

(event `E_SkillW_Collision`
  (params (Location :type "Vector Structure"))
  ;[1 1 1] Lou Skill W Collision 생성
  (`self.SpawnSkill_Location_ver` (`self.C_RefSkillW_Collision`) Location))

(fn `AllSpawnSkill`
  (params (SpawnSkillClass :type "Actor Class Reference") (GetWorldLocationTarget :type "SceneComponent Object Reference"))
  (returns (SpawnSkillReturnValue :type "Actor Object Reference"))
  ;[1 1 1] 마우스위치찾기+액터돌리기+스폰액터
  (`self.FindActorToMouseRotation`)
  (`self.TurnActor`)
  (bind _spawnskillreturnvalue (`self.SpawnSkill_Target_ver` SpawnSkillClass GetWorldLocationTarget))
  (return _spawnskillreturnvalue))

(fn `FindActorToMouseRotation`
  (bind (_returnvalue_x _returnvalue_y _returnvalue_z) (`KismetMathLibrary.BreakVector` (`self.K2_GetActorLocation`)))
  (bind (_returnvalue_x_2 _returnvalue_y_2) (`KismetMathLibrary.BreakVector` (`SceneComponent.K2_GetComponentLocation` (`self.CursorToWorld`))))
  ;[1 1 1 0] 액터와 마우스 사이의 회전값 저장
  (set `self.FindRotation` (`KismetMathLibrary.FindLookAtRotation` (`KismetMathLibrary.MakeVector` _returnvalue_x _returnvalue_y _returnvalue_z) (`KismetMathLibrary.MakeVector` _returnvalue_x_2 _returnvalue_y_2 _returnvalue_z))))

(fn `SaveCursorToWorld`
  (returns (Location :type "Vector Structure"))
  (bind (_bblockinghit _binitialoverlap _time _distance _location _impactpoint _normal _impactnormal) (`GameplayStatics.BreakHitResult` (`PlayerController.GetHitResultUnderCursorByChannel` (`GameplayStatics.GetPlayerController` 0) "TraceTypeQuery1" true)))
  (`SceneComponent.K2_SetWorldLocationAndRotation` (`self.CursorToWorld`) _location (`KismetMathLibrary.MakeRotationFromAxes` _impactnormal) false false)
  (return _location))

(fn `SkillVisibility`
  (params (Condition :type Boolean))
  (if Condition
    (`ActorComponent.SetActive` (`self.CharacterMovement`) false false)
    (`SceneComponent.SetVisibility` (`self.NP_LouSkillE`) true false)
    (else
      (`ActorComponent.SetActive` (`self.CharacterMovement`) true false)
      (`SceneComponent.SetVisibility` (`self.NP_LouSkillE`) false false))))

(fn `SpawnSkill_Location_ver`
  (params (SpawnSkillClass :type "Actor Class Reference") (Location :type "Vector Structure"))
  (returns (SpawnSkillReturnValue :type "Actor Object Reference"))
  (bind (_returnvalue_location _returnvalue_rotation _returnvalue_scale) (`KismetMathLibrary.BreakTransform` (`self.GetTransform`)))
  ;[1 1 1 0] 액터 스폰
  (bind _returnvalue (`|SpawnActorFromClass` SpawnSkillClass (`KismetMathLibrary.MakeTransform` Location _returnvalue_rotation _returnvalue_scale) "Undefined" "OverrideRootScale" self null))
  (return _returnvalue))

(fn `SpawnSkill_Target_ver`
  (params (SpawnSkillClass :type "Actor Class Reference") (GetWorldLocationTarget :type "SceneComponent Object Reference"))
  (returns (SpawnSkillReturnValue :type "Actor Object Reference"))
  (bind (_returnvalue_location _returnvalue_rotation _returnvalue_scale) (`KismetMathLibrary.BreakTransform` (`self.GetTransform`)))
  ;[1 1 1 0] 액터 스폰
  (bind _returnvalue (`|SpawnActorFromClass` SpawnSkillClass (`KismetMathLibrary.MakeTransform` (`SceneComponent.K2_GetComponentLocation` GetWorldLocationTarget) _returnvalue_rotation _returnvalue_scale) "Undefined" "OverrideRootScale" self null))
  (return _returnvalue))

(fn `SpawnSkillParticle`
  (params (SpawnLocation :type "Vector Structure") (Particle1 :type "NiagaraSystem Object Reference") (Particle2 :type "NiagaraSystem Object Reference") (Particle3 :type "NiagaraSystem Object Reference"))
  (returns (Particle1ReturnValue :type "NiagaraComponent Object Reference") (Particle2ReturnValue :type "NiagaraComponent Object Reference") (Particle3ReturnValue :type "NiagaraComponent Object Reference"))
  (bind _returnvalue (`NiagaraFunctionLibrary.SpawnSystemAtLocation` Particle1 SpawnLocation))
  (bind _returnvalue_2 (`NiagaraFunctionLibrary.SpawnSystemAtLocation` Particle2 SpawnLocation))
  (bind _returnvalue_3 (`NiagaraFunctionLibrary.SpawnSystemAtLocation` Particle3 SpawnLocation))
  (return _returnvalue _returnvalue_2 _returnvalue_3))

(fn `TurnActor`
  ;[1 1 1 0] 액터를 마우스 포인터의 방향으로 턴
  (`self.K2_SetActorRelativeRotation` (`self.FindRotation`)))

(fn `UserConstructionScript`)