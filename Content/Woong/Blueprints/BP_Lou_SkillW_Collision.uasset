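; Area collider for Lou's W skill that slows characters inside its sphere and destroys itself after a short fixed lifetime.
; Sphere begin overlap lowers the max walk speed of any character other than the owner, and end overlap sets a fixed higher speed, with no owner check.
; Both events test the capsule against the sphere, so overlaps from other components do not falsely toggle the slow.
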(event `self.ReceiveBeginPlay`
  ;[1 1 1] BeginPlay
  (`KismetSystemLibrary.Delay` 5.4)
  (`self.K2_DestroyActor`))

(event `self.Sphere.OnComponentBeginOverlap`
  (params (OverlappedComponent :type "PrimitiveComponent Object Reference") (OtherActor :type "Actor Object Reference") (OtherComp :type "PrimitiveComponent Object Reference") (OtherBodyIndex :type Integer) (bFromSweep :type Boolean) (SweepResult :type "HitResult Structure (by ref)"))
  ;[1 1 1] BeginOverlap
  (bind _ascharacter (cast `Character` OtherActor))
  (if (`PrimitiveComponent.IsOverlappingComponent` (`Character.CapsuleComponent` _ascharacter) (`self.Sphere`))
    (if (not (== _ascharacter (`self.GetOwner`)))
      (set `CharacterMovementComponent.MaxWalkSpeed` 150.0 (`Character.CharacterMovement` _ascharacter)))))

(event `self.Sphere.OnComponentEndOverlap`
  (params (OverlappedComponent :type "PrimitiveComponent Object Reference") (OtherActor :type "Actor Object Reference") (OtherComp :type "PrimitiveComponent Object Reference") (OtherBodyIndex :type Integer))
  ;[1 1 1] EndOverlap
  (bind _ascharacter (cast `Character` OtherActor))
  (if (not (`PrimitiveComponent.IsOverlappingComponent` (`Character.CapsuleComponent` _ascharacter) (`self.Sphere`)))
    (set `CharacterMovementComponent.MaxWalkSpeed` 300.0 (`Character.CharacterMovement` _ascharacter))))

(fn `UserConstructionScript`)