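; BP_Lou_SkillW is the actor for Lou's W skill, a spinning sphere that lasts two seconds or until it hits something.
; Either trigger calls ESkillWDead on the owning BP_Character_LOU, then destroys the actor; a failed owner cast skips both.
; Tick applies a fixed rotation step when the doubled frame delta passes a threshold, so spin speed depends on frame rate.
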(event `self.ReceiveTick`
  (params (DeltaSeconds :type "Float (single-precision)"))
  ;[1 1 1] Tick
  (set `self.Delta Seconds` (+ DeltaSeconds (`self.Delta Seconds`)))
  (if (>= (`self.Delta Seconds`) 0.014)
    (`SceneComponent.K2_AddRelativeRotation` (`self.Sphere`) (struct :`Pitch` 3.0 :`Roll` 5.0) false false)
    (set `self.Delta Seconds` 0.0)))

(event `self.ReceiveBeginPlay`
  ;[1 1 1] BeginPlay
  (`KismetSystemLibrary.Delay` 2.0)
  (bind _asbp_character_lou (cast `/Game/__OWNER/Woong/Character/Blueprints/BP_Character_LOU` (`self.GetOwner`) :!label _label))
  ;[1 1 1] BP_Character_Lou
  (`/Game/__OWNER/Woong/Character/Blueprints/BP_Character_LOU.E_SkillW_Dead` _asbp_character_lou)
  (`self.E_Destroy`))

(event `E_Destroy`
  (`self.K2_DestroyActor`))

(event `self.Sphere.OnComponentHit`
  (params (HitComponent :type "PrimitiveComponent Object Reference") (OtherActor :type "Actor Object Reference") (OtherComp :type "PrimitiveComponent Object Reference") (NormalImpulse :type "Vector Structure") (Hit :type "HitResult Structure (by ref)"))
  ;[1 1 1] 콜리전 Hit
  (goto _label))

(fn `UserConstructionScript`)